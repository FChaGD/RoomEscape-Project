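; BP_GI_GameInstance is the game instance that holds stage progress and manages the save game.
; On Init it loads the BP_S_SaveGame from its slot, or creates one if none exists.
; Events raise the open stage level, flag stages in a checker array, save with IsClear set, or delete the slot for a restart.
; Getters expose the stage state, main-stage entry value and slot name.
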(event `self.ReceiveInit`
  (bind _returnvalue (`GameplayStatics.DoesSaveGameExist` (`self.Save Slot Name`)))
  (if _returnvalue
    (bind _returnvalue_2 (`GameplayStatics.LoadGameFromSlot` (`self.Save Slot Name`)))
    (bind _asbp_s_save_game (cast `/Game/Save/BP_S_SaveGame` _returnvalue_2))
    (set `self.Save_Ref` _asbp_s_save_game)
    (else
      (bind _returnvalue_3 (`GameplayStatics.CreateSaveGameObject` "/Game/Save/BP_S_SaveGame.BP_S_SaveGame_C"))
      (set `self.Save_Ref` _returnvalue_3))))

(event `/Game/Map/Interface/BP_BPI_InstaceInfo.add Open Stage Level`
  (`/Engine/EditorBlueprintResources/StandardMacros.IncrementInt` (`self.Open Stage Level`)))

(event `/Game/Map/Interface/BP_BPI_InstaceInfo.set Save File`
  (bind _save_ref (`self.Save_Ref`))
  (set `/Game/Save/BP_S_SaveGame.isClear` true _save_ref)
  (`GameplayStatics.SaveGameToSlot` _save_ref (`self.Save Slot Name`)))

(event `/Game/Map/Interface/BP_BPI_InstaceInfo.Set StageChecker`
  (params (StageChecker :type Integer))
  (`KismetArrayLibrary.Array_Set` (`self.Stage Checker`) StageChecker true))

(event `/Game/Map/Interface/BP_BPI_InstaceInfo.set Restart`
  (`GameplayStatics.DeleteGameInSlot` (`self.Save Slot Name`)))

(fn `get Enter Main Stage`
  (returns (`Emter Main Stage` :type Integer))
  (return (`self.enter main stage`)))

(fn `get Open Stage Level`
  (returns (`Open Stage Level` :type Integer))
  (return (`self.Open Stage Level`)))

(fn `get Save Slot Name`
  (returns (SlotName :type String))
  (return (`self.Save Slot Name`)))

(fn `get StageChecker`
  (returns (NewParam :type "Array of Boolean"))
  (return (`self.Stage Checker`)))