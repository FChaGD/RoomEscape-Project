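; Player character blueprint that detects interactable objects in view and lets the player hold and drop one item.
; DetectForward line-traces from View, resolves the hit to its topmost parent actor, and shows or hides its prompt through BP_BPI_InterGrap.
; Held items are stored by class in the GrapActor child actor.
; Dropping spawns a BP_OB_Grapper of that class at the traced point; grabbing while holding first drops beneath the view.
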(event `/Game/Player/BP_BPI_Character.DetectForward`
  (bind _view (`self.View`))
  (bind _returnvalue (`SceneComponent.K2_GetComponentLocation` _view))
  (bind _outhit (`KismetSystemLibrary.LineTraceSingle` _returnvalue (+ _returnvalue (* (`KismetMathLibrary.GetForwardVector` (`SceneComponent.K2_GetComponentRotation` _view)) 300.0)) "TraceTypeQuery1"))
  ;[1 1 1] 기존 충돌 대상인지 검사
  (if (== (`.HitActor` (`GameplayStatics.BreakHitResult` (`self.View target`))) (`.HitActor` (`GameplayStatics.BreakHitResult` _outhit)))
    (bind (_bblockinghit _binitialoverlap _time _distance _location _impactpoint _normal _impactnormal _physmat _hitactor) (`GameplayStatics.BreakHitResult` (stale _output_get)))
    ;[1 1 1] 상호작용 UI 띄우기
    ;;[1 1 1] 새로운 히트 타겟 UI 띄우기
    (`/Engine/EditorBlueprintResources/StandardMacros.IsValid` _hitactor :!label _label
      (:`Is Valid`
        (bind _parentactor (`self.Target Child Checker` _hitactor))
        (if (`KismetSystemLibrary.DoesImplementInterface` _parentactor "/Game/Enviroment/Interface/BP_BPI_InterGrap.BP_BPI_InterGrap_C")
          (message `/Game/Enviroment/Interface/BP_BPI_InterGrap.ViewCheck` _parentactor self))))
    (else
      (`/Engine/EditorBlueprintResources/StandardMacros.IsValid` (`.HitActor` (`GameplayStatics.BreakHitResult` (`self.View target`)))
        (:`Is Valid`
          ;;[1 1 1] 상호작용 UI 끄기
          (bind _parentactor_2 (`self.Target Child Checker` (`.HitActor` (`GameplayStatics.BreakHitResult` (`self.View target`)))))
          (if (`KismetSystemLibrary.DoesImplementInterface` _parentactor_2 "/Game/Enviroment/Interface/BP_BPI_InterGrap.BP_BPI_InterGrap_C")
            (message `/Game/Enviroment/Interface/BP_BPI_InterGrap.TurnOffUI` _parentactor_2))
          (bind _output_get (set `self.View target` _outhit))
          (goto _label))
        (:`Is Not Valid`
          (bind _output_get_2 (set `self.View target` _outhit))
          (bind (_bblockinghit_2 _binitialoverlap_2 _time_2 _distance_2 _location_2 _impactpoint_2 _normal_2 _impactnormal_2 _physmat_2 _hitactor_2) (`GameplayStatics.BreakHitResult` _output_get_2))
          ;;[1 1 1] 첫 UI 타겟 띄우기
          (`/Engine/EditorBlueprintResources/StandardMacros.IsValid` _hitactor_2
            (:`Is Valid`
              (bind _parentactor_3 (`self.Target Child Checker` _hitactor_2))
              (if (`KismetSystemLibrary.DoesImplementInterface` _parentactor_3 "/Game/Enviroment/Interface/BP_BPI_InterGrap.BP_BPI_InterGrap_C")
                (message `/Game/Enviroment/Interface/BP_BPI_InterGrap.ViewCheck` _parentactor_3 self)))))))))

(event `/Game/Player/BP_BPI_Character.DestroygrappingObject`
  (bind _output_get (set `self.Grapping Object` "/Script/Engine.Actor"))
  (`ChildActorComponent.SetChildActorClass` (`self.GrapActor`) _output_get)
  (set `self.Grapping` false))

(event `/Game/Player/BP_BPI_Character.Grap`
  (params (Object :type "Actor Object Reference"))
  (bind _view (`self.View`))
  (bind _returnvalue (`SceneComponent.K2_GetComponentLocation` _view))
  (if (not (not (`self.Grapping`)))
    (bind _outhit (`KismetSystemLibrary.LineTraceSingle` _returnvalue (+ _returnvalue (* (`KismetMathLibrary.GetUpVector` (`SceneComponent.K2_GetComponentRotation` _view)) -300.0)) "TraceTypeQuery1"))
    (`/Engine/EditorBlueprintResources/StandardMacros.IsValid` (`.HitActor` (`GameplayStatics.BreakHitResult` _outhit))
      (:`Is Valid`
        (`self.Drop Item` _outhit))))
  (bind _output_get (set `self.Grapping Object` (`GameplayStatics.GetObjectClass` Object)))
  (`ChildActorComponent.SetChildActorClass` (`self.GrapActor`) _output_get)
  (`KismetSystemLibrary.Delay` 0.2)
  (set `self.Grapping` true))

(event `EnhancedInput|/Game/InputSystem/Input/IA_Grapping`
  (params (ActionValue :type Boolean) (ElapsedSeconds :type "Float (double-precision)") (TriggeredSeconds :type "Float (double-precision)") (InputAction :type "InputAction Object Reference" :default "/Game/InputSystem/Input/IA_Grapping.IA_Grapping"))
  (bind _view (`self.View`))
  (bind _returnvalue (`SceneComponent.K2_GetComponentLocation` _view))
  (:`Started`
    (if (`self.Grapping`)
      (bind _outhit (`KismetSystemLibrary.LineTraceSingle` _returnvalue (+ _returnvalue (* (`KismetMathLibrary.GetForwardVector` (`SceneComponent.K2_GetComponentRotation` _view)) 300.0)) "TraceTypeQuery1"))
      (`self.Drop Item` _outhit))))

(fn `Drop Item`
  (params (`View target` :type "HitResult Structure"))
  (bind _output_get (set `self.View target` `View target`))
  (bind (_bblockinghit _binitialoverlap _time _distance _location _impactpoint _normal _impactnormal _physmat _hitactor) (`GameplayStatics.BreakHitResult` _output_get))
  (`/Engine/EditorBlueprintResources/StandardMacros.IsValid` _hitactor
    (:`Is Valid`
      (`ChildActorComponent.SetChildActorClass` (`self.GrapActor`) "/Script/Engine.Actor")
      (bind _returnvalue (`|SpawnActorFromClass` "/Game/Enviroment/BP_OB_Grapper.BP_OB_Grapper_C" (`KismetMathLibrary.MakeTransform` _impactpoint) "AlwaysSpawn" "MultiplyWithRoot" null null))
      (`/Game/Enviroment/BP_OB_Grapper.Set Object Actor by class` _returnvalue (`self.Grapping Object`))
      (set `self.Grapping` false)
      (set `self.Grapping Object` (`GameplayStatics.GetObjectClass` _returnvalue))
      (set `self.View target` (struct)))))

(fn `Target Child Checker`
  (params (Target :type "Actor Object Reference"))
  (returns (ParentActor :type "Actor Object Reference"))
  (locals (tmp :type "Actor Object Reference") (loopCondition :type Boolean :default true))
  (bind _output_get (set `local.tmp` Target))
  (while (`local.loopCondition`)
    (if (`self.IsChildActor` _output_get)
      (set `local.tmp` (`self.GetParentActor` _output_get))
      (else
        (set `local.loopCondition` false))))
  (return (`local.tmp`)))

(fn `UserConstructionScript`)