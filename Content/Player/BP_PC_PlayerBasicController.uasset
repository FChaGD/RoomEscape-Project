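; Player controller that handles Enhanced Input movement and camera look for the controlled pawn.
; It adds the movement and acting mapping contexts on BeginPlay, then turns input into pawn movement and yaw/pitch rotation.
; Both inputs then send a forward-detection message to pawns implementing the character interface, for line tracing.
; Stop and restart events toggle a flag that gates movement and look input.
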(event `self.ReceiveBeginPlay`
  (bind _returnvalue (pcsubsystem `EnhancedInputLocalPlayerSubsystem` self))
  (`EnhancedInputSubsystemInterface.AddMappingContext` _returnvalue "/Game/InputSystem/IMC_Movement.IMC_Movement" 0 (struct))
  (`EnhancedInputSubsystemInterface.AddMappingContext` _returnvalue "/Game/InputSystem/IMC_Acting.IMC_Acting" 1 (struct)))

(event `EnhancedInput|/Game/InputSystem/Input/IA_Movement`
  (params (ActionValue :type "Vector2D Structure") (ElapsedSeconds :type "Float (double-precision)") (TriggeredSeconds :type "Float (double-precision)") (InputAction :type "InputAction Object Reference" :default "/Game/InputSystem/Input/IA_Movement.IA_Movement"))
  (bind (_x _y) (`KismetMathLibrary.BreakVector2D` ActionValue))
  (bind _returnvalue (`self.K2_GetPawn`))
  (bind _returnvalue_2 (`self.K2_GetPawn`))
  (:`Triggered`
    (if (`self.enable input`)
      ;[1 1 1] 좌우 조작
      (`Pawn.AddMovementInput` _returnvalue_2 (`self.GetActorRightVector` _returnvalue_2) _x false)
      ;[1 1 1] 앞뒤 조작
      (`Pawn.AddMovementInput` _returnvalue (`self.GetActorForwardVector` _returnvalue) _y false)
      ;[1 1 1] 라인 트레이스
      (if (`KismetSystemLibrary.DoesImplementInterface` (`self.K2_GetPawn`) "/Game/Player/BP_BPI_Character.BP_BPI_Character_C") :!label _label
        (message `/Game/Player/BP_BPI_Character.DetectForward` (`self.K2_GetPawn`))))))

(event `EnhancedInput|/Game/InputSystem/Input/IA_LookRotate`
  (params (ActionValue :type "Vector2D Structure") (ElapsedSeconds :type "Float (double-precision)") (TriggeredSeconds :type "Float (double-precision)") (InputAction :type "InputAction Object Reference" :default "/Game/InputSystem/Input/IA_LookRotate.IA_LookRotate"))
  (bind (_x _y) (`KismetMathLibrary.BreakVector2D` ActionValue))
  (:`Triggered`
    ;[1 1 1] 카메라 회전
    (if (`self.enable input`)
      (`Pawn.AddControllerYawInput` (`self.K2_GetPawn`) _x)
      (`Pawn.AddControllerPitchInput` (`self.K2_GetPawn`) _y)
      (goto _label))))

(event `/Game/Player/BP_BPI_PCCall.ReStart Player Input`
  (set `self.enable input` true))

(event `/Game/Player/BP_BPI_PCCall.Stop Player Input`
  (set `self.enable input` false))

(fn `UserConstructionScript`)