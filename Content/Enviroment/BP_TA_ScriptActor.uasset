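; BP_TA_ScriptActor is a one-shot trigger volume that adds a script entry when the main character enters it.
; On overlap it passes its ScriptTable and Key to the game mode's widget controller component, then destroys itself.
; On BeginPlay it removes itself if the game instance's open stage level message value has reached TargetLevel.
; The construction script scales the trigger box uniformly by Size.
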(event `self.ReceiveBeginPlay`
  (bind _open_stage_level (message `/Game/Map/Interface/BP_BPI_InstaceInfo.get Open Stage Level` (`GameplayStatics.GetGameInstance`)))
  (if (>= _open_stage_level (`self.Target Level`))
    (`self.K2_DestroyActor`)))

(event `self.Box.OnComponentBeginOverlap`
  (params (OverlappedComponent :type "PrimitiveComponent Object Reference") (OtherActor :type "Actor Object Reference") (OtherComp :type "PrimitiveComponent Object Reference") (OtherBodyIndex :type Integer) (bFromSweep :type Boolean) (SweepResult :type "HitResult Structure (by ref)"))
  (if (`.bSuccess` (cast `/Game/Player/BP_C_MainCharacter` OtherActor :!pure true))
    (`/Game/Widget/BP_SC_WidgetControllerComponent.Script Add` (`self.GetComponentByClass` (`GameplayStatics.GetGameMode`) "/Game/Widget/BP_SC_WidgetControllerComponent.BP_SC_WidgetControllerComponent_C") (`self.Script Table`) (`self.Key`))
    (`self.K2_DestroyActor`)))

(fn `UserConstructionScript`
  (bind _size (`self.Size`))
  (`SceneComponent.SetRelativeScale3D` (`self.Box`) (`KismetMathLibrary.MakeVector` _size _size _size)))