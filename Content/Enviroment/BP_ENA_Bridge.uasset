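; BP_ENA_Bridge is an environment bridge that stays hidden and non-solid until its Bridge event reveals it.
; The construction script hides the root hierarchy and disables the static mesh's collision.
; BeginPlay binds to a Bridge dispatcher, and the Bridge event unhides the hierarchy and restores query and physics collision.
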(event `self.ReceiveBeginPlay`
  (add `self.BridgeDispatcher` (`|CreateDelegate` :!event `Bridge`)))

(event `Bridge`
  (`SceneComponent.SetHiddenInGame` (`self.DefaultSceneRoot`) false true)
  (`PrimitiveComponent.SetCollisionEnabled` (`self.StaticMesh`) "QueryAndPhysics"))

(fn `UserConstructionScript`
  (`SceneComponent.SetHiddenInGame` (`self.DefaultSceneRoot`) true true)
  (`PrimitiveComponent.SetCollisionEnabled` (`self.StaticMesh`) "NoCollision"))