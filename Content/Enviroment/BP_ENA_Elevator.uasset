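; BP_ENA_Elevator is an environment elevator that raises a static mesh when the main character enters its box trigger.
; A timeline weight scaled by UpLength offsets the mesh's Z from a base location cached in the construction script.
; When the rise finishes, the timeline immediately reverses to lower it, and an activation flag blocks retriggering until the round trip ends.
; Debug prints remain on overlap, activation and each update.
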(event `self.Box.OnComponentBeginOverlap`
  (params (OverlappedComponent :type "PrimitiveComponent Object Reference") (OtherActor :type "Actor Object Reference") (OtherComp :type "PrimitiveComponent Object Reference") (OtherBodyIndex :type Integer) (bFromSweep :type Boolean) (SweepResult :type "HitResult Structure (by ref)"))
  (bind (_basevector_x _basevector_y _basevector_z) (`KismetMathLibrary.BreakVector` (`self.BaseVector`)))
  (`KismetSystemLibrary.PrintString` "박스 콜리전!!!!" true true (struct :`G` 0.66 :`B` 1.0 :`A` 1.0) 10.0)
  (cast `/Game/Player/BP_C_MainCharacter` OtherActor)
  (if (not (`self.IsActivatied`))
    (`KismetSystemLibrary.PrintString` "엘레베이터 실행!!" true true (struct :`G` 0.66 :`B` 1.0 :`A` 1.0) 10.0)
    (set `self.IsActivatied` true)
    (set `self.isUpping` true)
    (bind (_direction `_가중치`) (`Timeline|Elevator` :!label _label)
      (:`Update`
        (`KismetSystemLibrary.PrintString` "Hello")
        (`SceneComponent.K2_SetWorldLocation` (`self.StaticMesh`) (`KismetMathLibrary.MakeVector` _basevector_x _basevector_y (+ _basevector_z (* (`self.UpLength`) `_가중치`))) false false))
      (:`Finished`
        (if (`self.isUpping`)
          (set `self.isUpping` false)
          (goto _label :!via `Reverse`)
          (else
            (set `self.IsActivatied` false)))))))

(fn `UserConstructionScript`
  (set `self.BaseVector` (`SceneComponent.K2_GetComponentLocation` (`self.StaticMesh`))))