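; Actor component that shows an interactable's script lines, one per interaction.
; InitSetting supplies the interactor info and component order; Interaction clears and refills the script list through the GameMode's widget controller component.
; Each interaction advances the line index or flags the last line as final, passing updated info to the owner via the interactor interface.
; A specific order value shows the end script instead, and NextComponent returns a fixed enum value.
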(event `self.Interaction`
  (bind _returnvalue (`self.GetOwner`))
  (bind _returnvalue_2 (`self.GetOwner`))
  (bind (_info_scriptinfo _info_currentscriptnum _info_stagenum _info_ui _info_componentorder _info_componentindex _info_settingstage _info_endscrpit _info_isfinal _info_subkeyobject) (break `/Game/Enviroment/Struction/BP_ST_InteractorST` (`self.Info`)))
  (bind (_info_scriptinfo_2 _info_currentscriptnum_2 _info_stagenum_2 _info_ui_2 _info_componentorder_2 _info_componentindex_2 _info_settingstage_2 _info_endscrpit_2 _info_isfinal_2 _info_subkeyobject_2) (break `/Game/Enviroment/Struction/BP_ST_InteractorST` (`self.Info`)))
  (bind (_scriptinfo _currentscriptnum) (break `/Game/Enviroment/Struction/BP_ST_InteractorST` (`self.Info`)))
  (bind (_scriptinfo_2 _currentscriptnum_2) (break `/Game/Enviroment/Struction/BP_ST_InteractorST` (`self.Info`)))
  (bind (_scriptinfo_3 _currentscriptnum_3) (break `/Game/Enviroment/Struction/BP_ST_InteractorST` (`self.Info`)))
  (bind _returnvalue_3 (`Actor.GetComponentByClass` (`GameplayStatics.GetGameMode`) "/Game/Widget/BP_SC_WidgetControllerComponent.BP_SC_WidgetControllerComponent_C"))
  (bind _returnvalue_4 (`Actor.GetComponentByClass` (`GameplayStatics.GetGameMode`) "/Game/Widget/BP_SC_WidgetControllerComponent.BP_SC_WidgetControllerComponent_C"))
  (bind (_table _key) (break `/Game/Enviroment/Struction/BP_ST_ScriptObjectST` (`.Endscrpit_25_0E22BF3549DCFB3601A930B4E0D987D6` (break `/Game/Enviroment/Struction/BP_ST_InteractorST` (`self.Info`)))))
  (bind (_table_2 _key_2) (break `/Game/Enviroment/Struction/BP_ST_ScriptObjectST` (`|GetArrayItem` _scriptinfo_3 _currentscriptnum_3)))
  (bind (_table_3 _key_3) (break `/Game/Enviroment/Struction/BP_ST_ScriptObjectST` (`|GetArrayItem` _scriptinfo_2 _currentscriptnum_2)))
  ;[1 1 1] 스크립트 띄우기
  (if (`|EnumEquality` (`self.Component Order`) "NewEnumerator4")
    ;[1 1 1] 역할 다한 스크립트 출력
    (`/Game/Widget/BP_SC_WidgetControllerComponent.Clear Script List` _returnvalue_3)
    (`/Game/Widget/BP_SC_WidgetControllerComponent.Script Add` _returnvalue_3 _table _key)
    (elif (== (`KismetArrayLibrary.Array_Length` _scriptinfo) (+ _currentscriptnum 1))
      (`/Game/Widget/BP_SC_WidgetControllerComponent.Clear Script List` _returnvalue_4)
      (`/Game/Widget/BP_SC_WidgetControllerComponent.Script Add` _returnvalue_4 _table_2 _key_2)
      (set `self.Info` (make `/Game/Enviroment/Struction/BP_ST_InteractorST` _info_scriptinfo_2 _info_currentscriptnum_2 _info_stagenum_2 _info_ui_2 _info_componentorder_2 _info_componentindex_2 _info_settingstage_2 _info_endscrpit_2 true _info_subkeyobject_2))
      (if (`KismetSystemLibrary.DoesImplementInterface` _returnvalue "/Game/Enviroment/Interface/BP_BPI_InteractorInterface.BP_BPI_InteractorInterface_C")
        (message `/Game/Enviroment/Interface/BP_BPI_InteractorInterface.set Info` _returnvalue (`self.Info`) (`self.Component Order`)))
      (else
        (`/Game/Widget/BP_SC_WidgetControllerComponent.Clear Script List` _returnvalue_4)
        (`/Game/Widget/BP_SC_WidgetControllerComponent.Script Add` _returnvalue_4 _table_3 _key_3)
        (bind _output_get (set `self.Info` (make `/Game/Enviroment/Struction/BP_ST_InteractorST` _info_scriptinfo (+ _info_currentscriptnum 1) _info_stagenum _info_ui _info_componentorder _info_componentindex _info_settingstage _info_endscrpit _info_isfinal _info_subkeyobject)))
        (if (`KismetSystemLibrary.DoesImplementInterface` _returnvalue_2 "/Game/Enviroment/Interface/BP_BPI_InteractorInterface.BP_BPI_InteractorInterface_C")
          (message `/Game/Enviroment/Interface/BP_BPI_InteractorInterface.set Info` _returnvalue_2 _output_get (`self.Component Order`)))))))

(event `self.Init Setting`
  (params (Info :type "/Game/Enviroment/Struction/BP_ST_InteractorST Structure") (`Component Order` :type "/Game/Enviroment/Component/BP_ENM_ComponentType Enum" :default "NewEnumerator0"))
  ;[1 1 1] 정보 수령
  (set `self.Info` Info)
  (set `self.Component Order` `Component Order`))

(fn `Next Component`
  (returns (`next Component` :type "/Game/Enviroment/Component/BP_ENM_ComponentType Enum"))
  (return "NewEnumerator0"))