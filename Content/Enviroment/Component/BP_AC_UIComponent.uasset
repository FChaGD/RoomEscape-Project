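; BP_AC_UIComponent is an environment interaction component that shows a UI widget when interacted with.
; InitSetting stores an Info struct that supplies the widget class.
; Interaction creates that widget for the first player controller and hands it to the game mode's BP_SC_WidgetControllerComponent through ScreenWidget.
; NextComponent always returns a fixed enum value.
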(event `self.Init Setting`
  (params (Info :type "/Game/Enviroment/Struction/BP_ST_InteractorST Structure") (`Component Order` :type "/Game/Enviroment/Component/BP_ENM_ComponentType Enum" :default "NewEnumerator0"))
  ;[1 1 1] 정보 수령
  (set `self.Info` Info))

(event `self.Interaction`
  (bind _returnvalue (`|CreateWidget` (`.UI_9_3EB7E3724383A9171AD776A6740ADD8D` (break `/Game/Enviroment/Struction/BP_ST_InteractorST` (`self.Info`))) (`GameplayStatics.GetPlayerController` 0)))
  (`/Game/Widget/BP_SC_WidgetControllerComponent.Screen Widget` (`Actor.GetComponentByClass` (`GameplayStatics.GetGameMode`) "/Game/Widget/BP_SC_WidgetControllerComponent.BP_SC_WidgetControllerComponent_C") _returnvalue))

(fn `Next Component`
  (returns (`next Component` :type "/Game/Enviroment/Component/BP_ENM_ComponentType Enum"))
  (return "NewEnumerator0"))