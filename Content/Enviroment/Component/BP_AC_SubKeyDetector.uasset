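; BP_AC_SubKeyDetector is an interaction component for BP_OB_Interactor actors, apparently the detector for a sub-key object the player carries.
; InitSetting stores the supplied Info, which the graph does not otherwise use.
; Interaction sends DestroygrappingObjectMessage to player character 0, then casts the owner to BP_OB_Interactor and calls AddEndComponent on it.
; It performs no check on the held object, and BeginPlay and Tick are inactive.
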(event `self.Init Setting`
  (params (Info :type "/Game/Enviroment/Struction/BP_ST_InteractorST Structure") (`Component Order` :type "/Game/Enviroment/Component/BP_ENM_ComponentType Enum" :default "NewEnumerator0"))
  (set `self.Info` Info))

(event `self.Interaction`
  (message `/Game/Player/BP_BPI_Character.DestroygrappingObject` (`GameplayStatics.GetPlayerCharacter` 0))
  (bind _asbp_ob_interactor (cast `/Game/Enviroment/BP_OB_Interactor` (`self.GetOwner`)))
  (`/Game/Enviroment/BP_OB_Interactor.AddEndComponent` _asbp_ob_interactor))