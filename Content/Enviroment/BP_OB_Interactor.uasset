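; Interactable world object that delegates its behavior to actor components spawned from a class list at BeginPlay.
; A box overlap with the main character gates interaction, and ViewCheck shows a prompt widget.
; On IA_Interaction it passes InfoStruct to its components by class name, swapping script or UI components according to ComponentDirection.
; A passing stage-clear check sets the direction to End and adds a clear spawner.
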(event `self.ReceiveBeginPlay`
  (`self.Set Component`))

(event `Set Component`
  (for (_array_element _array_index) (`self.StartComponent`)
    (bind _returnvalue (`|AddComponentByClass` _array_element))
    (`KismetArrayLibrary.Array_Add` (`self.ComponentList`) _returnvalue)
    (if (== _array_index 1)
      (set `self.CurrentComponent` _array_element))))

(event `change component`
  (bind _componentlist (`self.ComponentList`))
  ;[1 1 1] 기능성 컴포넌트 교체
  (for _array_element (`self.ComponentList`)
    (switch `name` (`KismetStringLibrary.Conv_StringToName` (`KismetSystemLibrary.GetClassDisplayName` (`GameplayStatics.GetObjectClass` _array_element)))
      (:`BP_AC_ScriptComponet_C`
        _)
      (:`BP_AC_UIComponent_C`
        _))
    (`KismetArrayLibrary.Array_RemoveItem` _componentlist _array_element))
  (bind _returnvalue (`|AddComponentByClass` (`self.CurrentComponent`)))
  (`KismetArrayLibrary.Array_Add` _componentlist _returnvalue))

(event `self.Box.OnComponentBeginOverlap`
  (params (OverlappedComponent :type "PrimitiveComponent Object Reference") (OtherActor :type "Actor Object Reference") (OtherComp :type "PrimitiveComponent Object Reference") (OtherBodyIndex :type Integer) (bFromSweep :type Boolean) (SweepResult :type "HitResult Structure (by ref)"))
  (if (`.bSuccess` (cast `/Game/Player/BP_C_MainCharacter` OtherActor :!pure true))
    (set `self.Can InterAction` true)
    (`self.EnableInput` (`GameplayStatics.GetPlayerController` 0) :!label _label)))

(event `self.Box.OnComponentEndOverlap`
  (params (OverlappedComponent :type "PrimitiveComponent Object Reference") (OtherActor :type "Actor Object Reference") (OtherComp :type "PrimitiveComponent Object Reference") (OtherBodyIndex :type Integer))
  (if (`.bSuccess` (cast `/Game/Player/BP_C_MainCharacter` OtherActor :!pure true))
    (set `self.Can InterAction` false)
    (goto _label)))

(event `/Game/Enviroment/Interface/BP_BPI_InterGrap.ViewCheck`
  (params (Player :type "/Game/Player/BP_C_MainCharacter Object Reference"))
  ;[1 1 1] UI 띄우기
  (set `self.Player` Player)
  (if (and (`self.Can InterAction`) (not (`self.UIvisibility`)))
    (`self.EnableInput` (`GameplayStatics.GetPlayerController` 0))
    (`SceneComponent.SetVisibility` (`self.Widget`) true true)
    (set `self.UIvisibility` true)))

(event `/Game/Enviroment/Interface/BP_BPI_InterGrap.TurnOffUI`
  ;[1 1 1] UI 제거
  (`SceneComponent.SetVisibility` (`self.Widget`) false true)
  (set `self.UIvisibility` false)
  (`self.DisableInput` (`GameplayStatics.GetPlayerController` 0))
  (set `self.Player` null))

(event `EnhancedInput|/Game/InputSystem/Input/IA_Interaction`
  (params (ActionValue :type Boolean) (ElapsedSeconds :type "Float (double-precision)") (TriggeredSeconds :type "Float (double-precision)") (InputAction :type "InputAction Object Reference" :default "/Game/InputSystem/Input/IA_Interaction.IA_Interaction"))
  (bind (_infostruct_scriptinfo _infostruct_currentscriptnum _infostruct_stagenum _infostruct_ui _infostruct_componentorder _infostruct_componentindex _infostruct_settingstage _infostruct_endscrpit _infostruct_isfinal _infostruct_subkeyobject) (break `/Game/Enviroment/Struction/BP_ST_InteractorST` (`self.InfoStruct`)))
  (:`Started`
    (if (`self.Can InterAction`)
      (for _array_element (`self.ComponentList`)
        (switch `name` (`KismetStringLibrary.Conv_StringToName` (`KismetSystemLibrary.GetClassDisplayName` (`GameplayStatics.GetObjectClass` _array_element)))
          (:`BP_AC_StageClearChecker_C`
            ;[1 1 1] 스테이지 클리어 검사 컴포넌트
            (bind _stagechecker (`/Game/Enviroment/Component/BP_AC_StageClearChecker.StageChecking` (cast `/Game/Enviroment/Component/BP_AC_StageClearChecker` _array_element :!pure true) (`.StageNum_30_D0FC71E349CFF5CBA4540193D4BE9267` (break `/Game/Enviroment/Struction/BP_ST_InteractorST` (`self.InfoStruct`)))))
            (if _stagechecker
              (`self.AddEndComponent`)))
          (:`BP_AC_ScriptComponet_C`
            (switch `/Game/Enviroment/Component/BP_ENM_ComponentType` (`self.Component Direction`) :!label _label_2
              (:`NewEnumerator0`
                (bind _asbp_ac_base (cast `/Game/Enviroment/Component/BP_AC_Base` _array_element :!pure true))
                (`/Game/Enviroment/Component/BP_AC_Base.Init Setting` _asbp_ac_base (`self.InfoStruct`) "NewEnumerator0")
                (`/Game/Enviroment/Component/BP_AC_Base.Interaction` _asbp_ac_base))
              (:`NewEnumerator1`
                (`/Game/Enviroment/Component/BP_AC_Base.Init Setting` _asbp_ac_base (`self.InfoStruct`) "NewEnumerator1")
                (`/Game/Enviroment/Component/BP_AC_Base.Interaction` _asbp_ac_base)
                ;[1 1 1] 컴포넌트 변경
                (if (not (`.bSuccess` (cast `/Game/Enviroment/Component/BP_AC_ScriptComponet` _asbp_ac_base :!pure true)))
                  (set `self.CurrentComponent` "/Game/Enviroment/Component/BP_AC_ScriptComponet.BP_AC_ScriptComponet_C")
                  (`self.change component`)))
              (:`NewEnumerator4`
                ;[1 1 1] 컴포넌트 변경
                (if (not (`.bSuccess` (cast `/Game/Enviroment/Component/BP_AC_ScriptComponet` _asbp_ac_base :!pure true)))
                  (set `self.CurrentComponent` "/Game/Enviroment/Component/BP_AC_ScriptComponet.BP_AC_ScriptComponet_C")
                  (`self.change component`))
                (set `self.InfoStruct` (make `/Game/Enviroment/Struction/BP_ST_InteractorST` _infostruct_scriptinfo _infostruct_currentscriptnum _infostruct_stagenum _infostruct_ui _infostruct_componentorder _infostruct_componentindex _infostruct_settingstage _infostruct_endscrpit true _infostruct_subkeyobject))
                (`/Game/Enviroment/Component/BP_AC_Base.Init Setting` _asbp_ac_base (`self.InfoStruct`) (`self.Component Direction`))
                (`/Game/Enviroment/Component/BP_AC_Base.Interaction` _asbp_ac_base))))
          (:`BP_AC_UIComponent_C`
            (goto _label_2))
          (:`BP_AC_StageClearSpawner_C`
            (`/Game/Enviroment/Component/BP_AC_Base.Init Setting` _asbp_ac_base (`self.InfoStruct`) "NewEnumerator0")
            (`/Game/Enviroment/Component/BP_AC_Base.Interaction` _asbp_ac_base)))))))

(event `/Game/Enviroment/Interface/BP_BPI_InteractorInterface.set Info`
  (params (Info :type "/Game/Enviroment/Struction/BP_ST_InteractorST Structure") (`Component Order` :type "/Game/Enviroment/Component/BP_ENM_ComponentType Enum" :default "NewEnumerator0"))
  ;[1 1 1] 정보 갱신
  (set `self.InfoStruct` Info)
  (set `self.Component Direction` `Component Order`))

(fn `AddEndComponent`
  (set `self.Component Direction` "NewEnumerator4")
  (bind _returnvalue (`|AddComponentByClass` "/Game/Enviroment/Component/BP_AC_StageClearSpawner.BP_AC_StageClearSpawner_C"))
  (`KismetArrayLibrary.Array_Add` (`self.ComponentList`) _returnvalue))

(fn `UserConstructionScript`
  (`ChildActorComponent.SetChildActorClass` (`self.ChildActor`) (`self.Actor`))
  (`SceneComponent.SetVisibility` (`self.Widget`) false true))