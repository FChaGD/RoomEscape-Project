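; Trigger volume that records a stage clear when the player's main character enters its box.
; On BeginPlay it queries the Game Instance for the open stage level and destroys itself if that level has already reached TargetLevel.
; Otherwise, a box overlap with BP_C_MainCharacter passes ClearStage to the Game Instance's stage checker and destroys the trigger, making it one-shot.
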(event `self.ReceiveBeginPlay`
  (bind _open_stage_level (message `/Game/Map/Interface/BP_BPI_InstaceInfo.get Open Stage Level` (`GameplayStatics.GetGameInstance`)))
  (if (>= _open_stage_level (`self.Target Level`))
    (`self.K2_DestroyActor`)))

(event `self.Box.OnComponentBeginOverlap`
  (params (OverlappedComponent :type "PrimitiveComponent Object Reference") (OtherActor :type "Actor Object Reference") (OtherComp :type "PrimitiveComponent Object Reference") (OtherBodyIndex :type Integer) (bFromSweep :type Boolean) (SweepResult :type "HitResult Structure (by ref)"))
  (if (`.bSuccess` (cast `/Game/Player/BP_C_MainCharacter` OtherActor :!pure true))
    (message `/Game/Map/Interface/BP_BPI_InstaceInfo.set StageChecker` (`GameplayStatics.GetGameInstance`) (`self.Clear Stage`))
    (`self.K2_DestroyActor`)))

(fn `UserConstructionScript`)