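; Interactable pickup holder that displays a configurable child actor and lets the main character grab it with the IA_Grapping input.
; A box overlap sets the interaction flag and enables input, which the end overlap also enables while clearing the flag.
; ViewCheck stores the player and shows the prompt widget; TurnOffUI reverses this and disables input.
; Grabbing passes the child actor to the player's Grap, then destroys the holder.
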(event `self.ReceiveBeginPlay`
  (`KismetSystemLibrary.PrintString` (`KismetStringLibrary.Concat_StrStr` "오브젝트 배치 위치 : " (`KismetStringLibrary.Conv_VectorToString` (`SceneComponent.K2_GetComponentLocation` (`self.ChildActor`)))) true true (struct :`G` 0.66 :`B` 1.0 :`A` 1.0) 10.0))

(event `self.Box.OnComponentBeginOverlap`
  (params (OverlappedComponent :type "PrimitiveComponent Object Reference") (OtherActor :type "Actor Object Reference") (OtherComp :type "PrimitiveComponent Object Reference") (OtherBodyIndex :type Integer) (bFromSweep :type Boolean) (SweepResult :type "HitResult Structure (by ref)"))
  (if (`.bSuccess` (cast `/Game/Player/BP_C_MainCharacter` OtherActor :!pure true))
    (set `self.Can InterAction` true)
    (`self.EnableInput` (`GameplayStatics.GetPlayerController` 0) :!label _label)))

(event `self.Box.OnComponentEndOverlap`
  (params (OverlappedComponent :type "PrimitiveComponent Object Reference") (OtherActor :type "Actor Object Reference") (OtherComp :type "PrimitiveComponent Object Reference") (OtherBodyIndex :type Integer))
  (if (`.bSuccess` (cast `/Game/Player/BP_C_MainCharacter` OtherActor :!pure true))
    (set `self.Can InterAction` false)
    (goto _label)))

(event `/Game/Enviroment/Interface/BP_BPI_InterGrap.ViewCheck`
  (params (Player :type "/Game/Player/BP_C_MainCharacter Object Reference"))
  (set `self.Player` Player)
  (if (and (`self.Can InterAction`) (not (`self.UIvisibility`)))
    (`self.EnableInput` (`GameplayStatics.GetPlayerController` 0))
    (`SceneComponent.SetVisibility` (`self.Widget`) true true)
    (set `self.UIvisibility` true)))

(event `/Game/Enviroment/Interface/BP_BPI_InterGrap.TurnOffUI`
  (`SceneComponent.SetVisibility` (`self.Widget`) false true)
  (set `self.UIvisibility` false)
  (`self.DisableInput` (`GameplayStatics.GetPlayerController` 0))
  (set `self.Player` null))

(event `EnhancedInput|/Game/InputSystem/Input/IA_Grapping`
  (params (ActionValue :type Boolean) (ElapsedSeconds :type "Float (double-precision)") (TriggeredSeconds :type "Float (double-precision)") (InputAction :type "InputAction Object Reference" :default "/Game/InputSystem/Input/IA_Grapping.IA_Grapping"))
  (bind _player (`self.Player`))
  (:`Started`
    (if (`self.Can InterAction`)
      (`/Engine/EditorBlueprintResources/StandardMacros.IsValid` _player
        (:`Is Valid`
          (`/Game/Player/BP_C_MainCharacter.Grap` _player (`ChildActorComponent.ChildActor` (`self.ChildActor`)))
          (`self.K2_DestroyActor`))))))

(event `Set Object Actor by class`
  (params (NewParam :type "Actor Class Reference"))
  (bind _output_get (set `self.Actor` NewParam))
  (`ChildActorComponent.SetChildActorClass` (`self.ChildActor`) _output_get))

(fn `UserConstructionScript`
  (`ChildActorComponent.SetChildActorClass` (`self.ChildActor`) (`self.Actor`))
  (`SceneComponent.SetVisibility` (`self.Widget`) false true))